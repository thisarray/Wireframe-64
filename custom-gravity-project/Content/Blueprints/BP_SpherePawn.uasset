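; Pawn that moves sideways along the surface of an actor and jumps to other actors overhead, apparently spheres.
; Each tick a downward trace snaps it to the stored actor's impact point, taking only roll from the surface normal.
; Jump traces along the pawn's up vector; hitting a different actor teleports it there, blends the view target to that actor and stores it as the current surface.
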(event EventTick
  (params (DeltaSeconds :type Float%20%28single-precision%29))
  (bind _returnvalue (Transformation|GetActorLocation))
  (bind _returnvalue_2 (Transformation|GetActorRotation))
  (bind (_outhit _returnvalue_3) (Collision|LineTraceByChannel _returnvalue (+ _returnvalue (* (* (Transformation|GetActorUpVector) (Math|Float|MakeLiteralFloat -1.0)) (Math|Float|MakeLiteralFloat 5e+02))) "TraceTypeQuery1" false 0 "ForOneFrame"))
  (if _returnvalue_3
    (if (== (Variables|Default|GetStoredActor) (.HitActor (Collision|BreakHitResult _outhit)))
      (Transformation|SetActorTransform (Math|Transform|MakeTransform (.ImpactPoint (Collision|BreakHitResult _outhit)) (Math|Rotator|MakeRotator (.roll (Math|Rotator|MakeRotfromZX (.ImpactNormal (Collision|BreakHitResult _outhit)) (Transformation|GetActorForwardVector))) (.pitch _returnvalue_2) (.yaw _returnvalue_2)) "1.000000,1.000000,1.000000")))))

(event Input|ActionEvents|InputActionJump
  (params (Key :type Key%20Structure :default "None"))
  (bind _returnvalue (Transformation|GetActorLocation))
  (bind _returnvalue_2 (Transformation|GetActorRotation))
  (:Pressed
    (bind (_outhit _returnvalue_3) (Collision|LineTraceByChannel _returnvalue (+ _returnvalue (* (Transformation|GetActorUpVector) (Math|Float|MakeLiteralFloat 7.5e+02))) "TraceTypeQuery1" false 0 "ForOneFrame"))
    (if _returnvalue_3
      (if (not (== (Variables|Default|GetStoredActor) (.HitActor (Collision|BreakHitResult _outhit))))
        (Transformation|SetActorTransform (Math|Transform|MakeTransform (.ImpactPoint (Collision|BreakHitResult _outhit)) (Math|Rotator|MakeRotator (.roll (Math|Rotator|MakeRotfromZX (.ImpactNormal (Collision|BreakHitResult _outhit)) (Transformation|GetActorForwardVector))) (.pitch _returnvalue_2) (.yaw _returnvalue_2)) "1.000000,1.000000,1.000000"))
        (Game|Player|SetViewTargetwithBlend (Game|GetPlayerController 0) (.HitActor (Collision|BreakHitResult _outhit)) 0.1 "VTBlend_Linear" 0.0 false)
        (Variables|Default|SetStoredActor (.HitActor (Collision|BreakHitResult _outhit)))))))

(event Input|AxisEvents|InputAxisMoveRight/Left
  (params (AxisValue :type Float%20%28single-precision%29))
  (Pawn|Input|AddMovementInput (Transformation|GetActorRightVector) AxisValue false))

(fn ConstructionScript)